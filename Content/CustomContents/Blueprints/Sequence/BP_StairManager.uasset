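; BP_StairManager switches a set of stair actors on or off in sequence through two events, StairActivate and StairDeactivate.
; Both pass ArrayActors to the SequenceManager's RequestSequential and differ only in the activate flag and debug message.
; The interval is Duration divided by the actor count, guarded against an empty array, and Duration itself is also passed along.
; Each event prints its "Done" message straight after issuing the request.
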(event Custom|Stair%20Activate
  (Class|SequenceManager|RequestSequential (Subsystems|GetSequenceManager) (Variables|Default|GetArrayActors) true 0.0 (/ (Variables|Default|GetDuration) (Math|Integer|Max(Integer) (Utilities|Array|Length (Variables|Default|GetArrayActors)) 1)) (Variables|Default|GetDuration))
  (Development|PrintString "Activate Done"))

(event Custom|Stair%20Deactivate
  (Class|SequenceManager|RequestSequential (Subsystems|GetSequenceManager) (Variables|Default|GetArrayActors) false 0.0 (/ (Variables|Default|GetDuration) (Math|Integer|Max(Integer) (Utilities|Array|Length (Variables|Default|GetArrayActors)) 1)) (Variables|Default|GetDuration))
  (Development|PrintString "Deactivate Done"))

(fn ConstructionScript)
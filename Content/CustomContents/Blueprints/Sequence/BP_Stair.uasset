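; BP_Stair is a stair Blueprint with a static mesh that appears and disappears through Activate and Deactivate events.
; Activate unhides the mesh and Deactivate hides it, each without propagating to child components.
; Both events print a debug string with the object name and event name; Activate's Duration is only printed, so the visibility change is immediate.
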(event EventActivate
  (params (Duration :type Float%20%28single-precision%29))
  (Development|PrintString (Utilities|String|Append (Utilities|GetDisplayName self) "|" (Utilities|String|ToString(Float) Duration) "|" "Activate"))
  (Development|SetHiddeninGame (Variables|Default|GetStaticMesh) false false))

(event EventDeactivate
  (Development|PrintString (Utilities|String|Append (Utilities|GetDisplayName self) "|" (Utilities|String|ToString(Float) 0.0) "|" "Deactivate"))
  (Development|SetHiddeninGame (Variables|Default|GetStaticMesh) true false))

(fn ConstructionScript)
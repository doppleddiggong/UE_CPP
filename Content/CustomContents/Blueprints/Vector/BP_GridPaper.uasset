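; BP_GridPaper is a grid paper Blueprint that animates a point between Start and End positions on a repeating five-second loop.
; Tick counts Duration down and resets it when it drops below zero, so the point travels from End toward Start, then jumps back.
; An ease-in interpolation on the remaining-time fraction gives the position, whose X and Y are truncated to integers and passed to UpdatePointLocation.
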(event EventTick
  (params (DeltaSeconds :type Float%20%28single-precision%29))
  (bind _output_get (Variables|Default|SetDuration (- (Variables|Default|GetDuration) DeltaSeconds)))
  (if (< _output_get 0.0)
    (Variables|Default|SetDuration 5.0))
  (Class|GridPaper|UpdatePointLocation (Utilities|Struct|MakeIntVector2 (Math|Float|Truncate (.x (Math|Interpolation|Ease "EaseIn" (/ (Variables|Default|GetDuration) 5.0) (Variables|Default|Getstart) (Variables|Default|Getend) 2.0))) (Math|Float|Truncate (.y (Math|Interpolation|Ease "EaseIn" (/ (Variables|Default|GetDuration) 5.0) (Variables|Default|Getstart) (Variables|Default|Getend) 2.0))))))

(event EventBeginPlay
  (Variables|Default|SetDuration 5.0))

(fn ConstructionScript)
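; BP_GeometryParabola is an actor that moves along a geometric parabolic arc from its spawn location to a point offset along world Y, apparently a demo of the Parabola component.
; BeginPlay registers the "Geometry" track with that component and briefly draws its path for debugging.
; Each Tick sets the actor location from the track and smoothly interpolates its rotation toward the direction of travel with RInterpTo.
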(event EventBeginPlay
  ;[0.15 0.15 0.15 0.5] Comment
  (bind _output_get (Variables|Default|SetGeometry (Utilities|Struct|MakeParabolaGeometricTrack (Transformation|GetActorLocation) (+ (Transformation|GetActorLocation) "0.000000,1400.000000,0.000000") (Variables|Default|GetDuration) 2e+02 "0.000000,0.000000,1.000000" false 0.0)))
  (Class|ParabolaComponent|SetGeometricParabolaTrack (Variables|Default|GetParabola) "Geometry" _output_get)
  (Class|ParabolaComponent|DrawGeometricPath (Variables|Default|GetParabola) "Geometry" 30 (Variables|Default|GetColor) 5.0))

(event EventTick
  (params (DeltaSeconds :type Float%20%28single-precision%29))
  (Transformation|SetActorLocation (Class|ParabolaComponent|GetGeometricParabolaVectorTrack (Variables|Default|GetParabola) "Geometry") false false)
  (Transformation|SetActorRotation (Math|Interpolation|RInterpTo (Transformation|GetActorRotation) (Class|ParabolaComponent|GetParabolaFacing (Variables|Default|GetParabola) "Geometry" false "X") (Utilities|Time|GetWorldDeltaSeconds) 12.0)))

(fn ConstructionScript)
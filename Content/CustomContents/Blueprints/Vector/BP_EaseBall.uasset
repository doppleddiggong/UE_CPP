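; BP_EaseBall is an actor that moves from StartPos to EndPos with a bouncing in-out ease.
; BeginPlay registers a MovePos vector track on Ease, timed by Delay.
; Tick reads that track and sets the actor location without sweep.
; A separate UpdatePos event eases manually by EaseType, but nothing here calls it and its countdown subtracts zero.
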(event Custom|UpdatePos
  ;[0.15 0.15 0.15 0.5] UpdatePos Ease
  (bind _output_get (Variables|Default|SetDuration (- (Variables|Default|GetDuration) 0.0)))
  (if (< _output_get 0.0)
    (Variables|Default|SetDuration 5.0))
  (Transformation|SetActorLocation (Math|Interpolation|Ease (Variables|Default|GetEaseType) (/ (Variables|Default|GetDuration) (Variables|Default|GetDelay)) (Variables|Default|GetStartPos) (Variables|Default|GetEndPos) 2.0) false false))

(event EventTick
  (params (DeltaSeconds :type Float%20%28single-precision%29))
  ;[0.15 0.15 0.15 0.5] Tick
  (Transformation|SetActorLocation (Class|EaseComponent|GetEaseVectorTrack (Variables|Default|GetEase) "MovePos") false false))

(event EventBeginPlay
  ;[0.15 0.15 0.15 0.5] Begin
  (Variables|Default|SetDuration (Variables|Default|GetDelay))
  (Class|EaseComponent|SetEaseVectorTrack (Variables|Default|GetEase) "MovePos" "EaseInOutBounce" (Variables|Default|GetStartPos) (Variables|Default|GetEndPos) (Variables|Default|GetDelay)))

(fn ConstructionScript)
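; BP_BallisticParabola is an actor that flies along a ballistic arc, apparently a sample of a parabola track component.
; On BeginPlay it registers a "Ballistic" track on its Parabola component from its location, duration, gravity and launch direction and speed, then draws the path briefly for debugging.
; Each Tick it moves to the track's current position and smoothly interpolates its rotation to face along the curve, including pitch.
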(event EventBeginPlay
  ;[0.15 0.15 0.15 0.5] Comment
  (bind _output_get (Variables|Default|SetGeometry (Utilities|Struct|MakeParabolaBallisticTrack (Transformation|GetActorLocation) (Variables|Default|GetDuration) -9.8e+02 "0.500000,0.866000,0.000000" 1.2e+03 false 0.0)))
  (Class|ParabolaComponent|SetBallisticParabolaTrack (Variables|Default|GetParabola) "Ballistic" _output_get)
  (Class|ParabolaComponent|DrawBallisticPath (Variables|Default|GetParabola) "Ballistic" 30 (Variables|Default|GetColor) 5.0))

(event EventTick
  (params (DeltaSeconds :type Float%20%28single-precision%29))
  (Transformation|SetActorLocation (Class|ParabolaComponent|GetBallisticParabolaVectorTrack (Variables|Default|GetParabola) "Ballistic") false false)
  (Transformation|SetActorRotation (Math|Interpolation|RInterpTo (Transformation|GetActorRotation) (Class|ParabolaComponent|GetParabolaFacing (Variables|Default|GetParabola) "Ballistic" false "X") (Utilities|Time|GetWorldDeltaSeconds) 12.0)))

(fn ConstructionScript)
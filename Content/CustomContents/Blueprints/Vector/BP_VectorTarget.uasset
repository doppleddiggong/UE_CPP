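; BP_VectorTarget is an actor that turns to face the player's third-person character every tick, apparently as a vector math demo.
; It caches the character on BeginPlay, then draws debug line traces forward and at 45 degrees either side, ignoring their hits.
; It prints the dot-product angle between its forward vector and the direction to the player.
; A debug cone draw is present but never runs.
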(event EventBeginPlay
  (bind _asbp_third_person_character (Utilities|Casting|CastToBP_ThirdPersonCharacter (Game|Player|GetPlayerPawn 0)))
  (Variables|Default|SetAs%20BP%20Third%20Person%20Character _asbp_third_person_character))

(event EventTick
  (params (DeltaSeconds :type Float%20%28single-precision%29))
  (bind _returnvalue (Transformation|GetActorLocation))
  (Transformation|SetActorRotation (Math|Rotator|MakeRotfromX (- (Transformation|GetActorLocation (Variables|Default|GetAs%20BP%20Third%20Person%20Character)) (Transformation|GetActorLocation))))
  (Collision|LineTraceByChannel _returnvalue (+ _returnvalue (* (Math|Vector|GetForwardVector (Transformation|GetActorRotation)) 1e+03)) "TraceTypeQuery1" false 0 "ForDuration" true "(R=0.555617,G=0.007296,B=1.000000,A=1.000000)" "(R=0.000000,G=1.000000,B=0.000000,A=1.000000)" 0.0)
  (Collision|LineTraceByChannel _returnvalue (+ (Transformation|GetActorLocation) (* (Math|Vector|RotateVector (Math|Vector|GetForwardVector (Transformation|GetActorRotation)) (Math|Rotator|MakeRotator 0.0 0.0 -45.0)) 1e+03)) "TraceTypeQuery1" false 0 "ForDuration" true "(R=0.000000,G=0.651670,B=1.000000,A=1.000000)" "(R=0.000000,G=1.000000,B=0.000000,A=1.000000)" 0.0)
  (Collision|LineTraceByChannel _returnvalue (+ (Transformation|GetActorLocation) (* (Math|Vector|RotateVector (Math|Vector|GetForwardVector (Transformation|GetActorRotation)) (Math|Rotator|MakeRotator 0.0 0.0 45.0)) 1e+03)) "TraceTypeQuery1" false 0 "ForDuration" true "(R=0.000000,G=0.651670,B=1.000000,A=1.000000)" "(R=0.000000,G=1.000000,B=0.000000,A=1.000000)" 0.0)
  (Development|PrintString (Utilities|String|ToString(Float) (Class|KismetMathLibrary|DegAcos (Math|Vector|DotProduct (Transformation|GetActorForwardVector) (Math|Vector|Normalize (- (Transformation|GetActorLocation (Variables|Default|GetAs%20BP%20Third%20Person%20Character)) (Transformation|GetActorLocation))))))))

(fn ConstructionScript)